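; Hydra motion-controller actor that drives a pool stick and the player character's shooting.
; The first trigger press enables tracking and stores an initial stick rotation, which this graph never reads back.
; While enabled, movement of the hand-0 controller copies its raw position and rotation straight onto the PoolStick.
; Later presses call SetShooting on MyCharacter, and every trigger release calls SetDoneShooting.
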(event EventHydraControllerMoved
  (params (Controller :type Integer) (Position :type Vector :default "0, 0, 0") (Velocity :type Vector :default "0, 0, 0") (Acceleration :type Vector :default "0, 0, 0") (Rotation :type Rotator :default "0, 0, 0"))
  ;[1 1 1] Move Pool Stick
  (if (Variables|Default|GetHydraEnabled)
    (bind _returnvalue (Class|HydraPluginActor|HydraWhichHand Controller))
    (if (== _returnvalue 0)
      (Utilities|Casting|CastToMyCharacter (Game|GetPlayerCharacter 0))
      (Transformation|SetActorTransform (Variables|Default|GetpoolStick) (Math|Transform|MakeTransform Position Rotation)))))

(event EventHydraTriggerPressed
  (params (Controller :type Integer))
  (if (Variables|Default|GetHydraEnabled)
    (bind _asmycharacter_c (Utilities|Casting|CastToMyCharacter (Game|GetPlayerCharacter 0)))
    (Default|SetShooting _asmycharacter_c)
    (else
      (Variables|Default|SetHydraEnabled true)
      (Variables|Default|SetInitialPoolStickRotation (stale EventHydraControllerMoved Rotation)))))

(event EventHydraTriggerReleased
  (params (Controller :type Integer))
  (bind _asmycharacter_c (Utilities|Casting|CastToMyCharacter (Game|GetPlayerCharacter 0)))
  (Default|SetDoneShooting _asmycharacter_c))

(fn ConstructionScript)